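; Chair display actor that shows a swappable product mesh, likely for a mobile AR-style viewer.
; Construction applies the mesh and plate scale from a product reference and hides the plate.
; Tick yaws the actor from device rotation rate and rebinds the main menu's change event, which cycles meshes through data table rows.
; SetChairPosition deprojects a screen point and traces to move the scene component onto the Plane actor.
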(event `self.ReceiveBeginPlay`
  ; Heejung
  (`StaticMeshComponent.SetStaticMesh` (`self.StaticMesh`) null))

(event `self.ReceiveTick`
  (params (DeltaSeconds :type "Float (single-precision)"))
  (`self.K2_AddActorLocalRotation` (`KismetMathLibrary.MakeRotator` 0.0 0.0 (* (* (.x (`.RotationRate` (`PlayerController.GetInputMotionState` (`GameplayStatics.GetPlayerController` 0)))) -1.0) (`GameplayStatics.GetWorldDeltaSeconds`) 100.0)))
  ; Heejung
  (add `self.ChangeObject` (`/Game/BP_Chair_HJ.BP_ChangeObject_HJ` (`.MainMenu` (`self.MainMenu`))) (delegate `ChangeObject`)))

(event `ChangeObject`
  ; Heejung
  (if (> (`self.ObjectNumber`) 2)
    (set `self.ObjectNumber` 0)
    (else
      (set `self.ObjectNumber` (+ (`self.ObjectNumber`) 1))))
  (bind _outrownames (`DataTableFunctionLibrary.GetDataTableRowNames` null))
  (bind _returnvalue (`|GetDataTableRow` null (`|GetArrayItem` _outrownames (`self.ObjectNumber`)))
    (:`then`
      (`StaticMeshComponent.SetStaticMesh` (`self.StaticMesh`) (`.Mesh_6_4AD7BB5B4A0DE523769763BB29BCE888` (break `` _returnvalue))))))

(fn `AssignProductAsset`
  (bind _plate (`/Game/Blueprint/Ref.Plate` (`self.Ref`)))
  (`StaticMeshComponent.SetStaticMesh` (`self.StaticMesh`) (`.StaticMesh` (`/Game/Blueprint/Ref.StaticMesh` (`self.Ref`))))
  (`SceneComponent.SetWorldScale3D` (`self.Plate`) (`KismetMathLibrary.MakeVector` _plate _plate))
  (`SceneComponent.SetVisibility` (`self.Plate`) false false))

(fn `SetChairPosition`
  (params (Location :type "Vector2D Structure"))
  (bind (_worldposition _worlddirection) (`GameplayStatics.DeprojectScreenToWorld` (`GameplayStatics.GetPlayerController` 0) Location))
  (bind (_outhit _returnvalue) (`KismetSystemLibrary.LineTraceSingleForObjects` _worldposition (+ _worldposition (* _worlddirection 1000.0)) (`|MakeArray` "ObjectTypeQuery1" "ObjectTypeQuery2" "ObjectTypeQuery3" "ObjectTypeQuery4" "ObjectTypeQuery5" "ObjectTypeQuery6" :!type "EObjectTypeQuery Enum")))
  (if _returnvalue
    (bind (_bblockinghit _binitialoverlap _time _distance _location _impactpoint _normal _impactnormal _physmat _hitactor) (`GameplayStatics.BreakHitResult` _outhit))
    (if (== _hitactor (`self.Plane`))
      (`SceneComponent.K2_SetWorldLocation` (`self.Scene`) _location false false))))

(fn `UserConstructionScript`
  (`self.AssignProductAsset`))