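; BP_Chair is a placeable chair product actor that is moved and rotated from screen-space input.
; Construction applies the first mesh from its Ref data, then scales and hides the Plate component.
; Positioning deprojects a screen point into a line trace and moves the Scene component to the hit only on the Plane actor.
; Rotation yaws Scene by negated horizontal Direction while accumulating the 2D distance travelled by the input location.
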(fn `AssignProductAsset`
  (bind _ref (`self.Ref`))
  (bind _plate (`/Game/Blueprint/Ref.Plate` _ref))
  (`StaticMeshComponent.SetStaticMesh` (`self.StaticMesh`) (`|GetArrayItem` (`/Game/Blueprint/Ref.StaticMesh` _ref)))
  (`SceneComponent.SetWorldScale3D` (`self.Plate`) (`KismetMathLibrary.MakeVector` _plate _plate))
  (`SceneComponent.SetVisibility` (`self.Plate`) false false))

(fn `SetChairPosition`
  (params (Location :type "Vector2D Structure"))
  (bind (_worldposition _worlddirection) (`GameplayStatics.DeprojectScreenToWorld` (`GameplayStatics.GetPlayerController` 0) Location))
  (bind (_outhit _returnvalue) (`KismetSystemLibrary.LineTraceSingleForObjects` _worldposition (+ _worldposition (* _worlddirection 1000.0)) (`|MakeArray` "ObjectTypeQuery1" "ObjectTypeQuery2" "ObjectTypeQuery3" "ObjectTypeQuery4" "ObjectTypeQuery5" "ObjectTypeQuery6" :!type "EObjectTypeQuery Enum")))
  (if _returnvalue
    (bind (_bblockinghit _binitialoverlap _time _distance _location _impactpoint _normal _impactnormal _physmat _hitactor) (`GameplayStatics.BreakHitResult` _outhit))
    (if (== _hitactor (`self.Plane`))
      (`SceneComponent.K2_SetWorldLocation` (`self.Scene`) _location false false))))

(fn `SetChairRotation`
  (params (Location :type "Vector2D Structure") (Direction :type "Vector2D Structure"))
  (set `self.Distance` (+ (`KismetMathLibrary.Distance2D` (`local.Location`) (`self.PreviousLocation`)) (`self.Distance`)))
  (set `self.PreviousLocation` (`local.Location`))
  (`SceneComponent.K2_AddRelativeRotation` (`self.Scene`) (`KismetMathLibrary.MakeRotator` 0.0 0.0 (* (`KismetMathLibrary.BreakVector2D` (`local.Direction`)) -1.0)) false false))

(fn `UserConstructionScript`
  (`self.AssignProductAsset`))