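; AR player pawn for placing and manipulating a chair on detected planes, with an IKEA-style main menu.
; After scanning, Tick periodically traces from screen center to refresh a candidate plane actor sized to the AR geometry.
; Touch traces select a plane, then spawn BP_Chair on it and hide it.
; Timed gesture recognition in Tick drives chair movement from a held finger and rotation from two fingers; ResetPlace clears the placement.
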(event `InputTouch`
  (params (Location :type "Vector Structure") (FingerIndex :type "ETouchIndex Enum"))
  (bind _selectedplane (`self.SelectedPlane`))
  (:`Pressed`
    (switch `ETouchIndex` FingerIndex
      (:`Touch1`
        (if (`self.PlaneIsSelected`)
          (if (not (`self.ObjectIsPlaced`))
            (bind (_outhit _returnvalue) (`self.WorldHit` (`self.TouchLocation`)))
            (if _returnvalue
              (bind (_bblockinghit _binitialoverlap _time _distance _location _impactpoint _normal _impactnormal _physmat _hitactor) (`GameplayStatics.BreakHitResult` _outhit))
              (if (== (`self.SelectedPlane`) _hitactor)
                (bind _returnvalue_2 (`|SpawnActorFromClass` "/Game/Blueprint/BP_Chair.BP_Chair_C" (`KismetMathLibrary.Conv_VectorToTransform` _location) "Undefined" "MultiplyWithRoot" null null))
                (bind _output_get (set `self.Object` _returnvalue_2))
                (set `/Game/Blueprint/BP_Chair.Plane` _selectedplane _output_get)
                (set `self.ObjectIsPlaced` true)
                (`/Game/Blueprint/BP_Plane.Hide` _selectedplane)
                (`self.ARObjectSpawned`))))
          (else
            (bind (_outhit_2 _returnvalue_3) (`self.WorldHit` (`self.TouchLocation`)))
            (if _returnvalue_3
              (bind _asbp_plane (cast `/Game/Blueprint/BP_Plane` (`.HitActor` (`GameplayStatics.BreakHitResult` _outhit_2))))
              (`/Engine/EditorBlueprintResources/StandardMacros.IsValid` (`/Game/Blueprint/BP_Plane.Plane` _asbp_plane)
                (:`Is Valid`
                  (bind _output_get_2 (set `self.SelectedPlane` _asbp_plane))
                  (`self.BPPlaneSelected` _output_get_2)
                  (set `self.PlaneIsSelected` true))))))))))

(event `self.ReceiveBeginPlay`
  ; 여기 메인 위젯
  (bind _returnvalue (`|CreateWidget` "/Game/UI/ikea/BP_IkeaMainMenu.BP_IkeaMainMenu_C" (`GameplayStatics.GetPlayerController` 0)))
  (bind _output_get (set `self.Main` _returnvalue))
  (`UserWidget.AddToViewport` _output_get 0))

(event `self.ReceiveTick`
  (params (DeltaSeconds :type "Float (single-precision)"))
  (set `self.Delta` DeltaSeconds)
  (`|ExecutionSequence`
    (:`then_0`
      (`self.GestureReset`)
      (`self.GestureRecognition`)
      (`self.TwoTouch`)
      (if (`self.GestureRecognize`)
        (switch `/Game/Blueprint/E_State` (`self.State`)
          (:`NewEnumerator0`
            (`/Game/Blueprint/BP_Chair.SetChairPosition` (`self.Object`) (`self.TouchLocation`)))
          (:`NewEnumerator1`
            (`/Game/Blueprint/BP_Chair.SetChairRotation` (`self.Object`) (`self.TouchLocation`) (`self.FingerDirection`))))))
    (:`then_1`
      (if (and (`self.ScanningIsDone`) (not (`self.PlaneIsSelected`)))
        (bind _output_get (set `self.ShowPlaneTimer` (+ (`self.Delta`) (`self.ShowPlaneTimer`))))
        (if (> _output_get 1.0)
          (set `self.ShowPlaneTimer` 0.0)
          (`self.Update`))))))

(event `InputAction|Finger`
  (params (Key :type "Key Structure"))
  (:`Pressed`
    (bind _outhit (`self.WorldHit` (`self.TouchLocation`)))
    (cast `/Game/Blueprint/BP_Chair` (`.HitActor` (`GameplayStatics.BreakHitResult` _outhit)))
    (set `self.FingerPressed` true)
    (set `self.FingerTimer` 0.0))
  (:`Released`
    (set `self.FingerPressed` false)))

(event `InputAction|TwoFinger`
  (params (Key :type "Key Structure"))
  (:`Pressed`
    (set `self.TwoFingerPressed` true)
    (set `self.TwoFingerTimer` 0.0)
    (bind _output_get (set `self.PreviousFingerPosition` (`self.TouchLocation`)))
    (set `self.StartingFingerPosition_0` _output_get)
    (set `self.PreviousFingerDistance` (`self.FingerDistance`)))
  (:`Released`
    (set `self.TwoFingerPressed` false)))

(fn `Create`
  (params (ARPlane :type "ARPlaneGeometry Object Reference"))
  (returns (Plane :type "/Game/Blueprint/BP_Plane Object Reference"))
  (bind _returnvalue (`|SpawnActorFromClass` "/Game/Blueprint/BP_Plane.BP_Plane_C" (`ARTrackedGeometry.GetLocalToWorldTransform` ARPlane) "Undefined" "MultiplyWithRoot" null null))
  (`SceneComponent.SetRelativeScale3D` (`/Game/Blueprint/BP_Plane.Plane` _returnvalue) (`KismetMathLibrary.MakeVector` (.x (/ (`ARPlaneGeometry.GetExtent` ARPlane) 50.0)) (.y (/ (`ARPlaneGeometry.GetExtent` ARPlane) 50.0))))
  (return _returnvalue))

(fn `FingerDirection`
  (returns (ReturnValue :type "Vector2D Structure"))
  (bind (_locationx _locationy) (`PlayerController.GetInputTouchState` (`GameplayStatics.GetPlayerController` 0) "Touch1"))
  (return (`KismetMathLibrary.Normal2D` (- (`KismetMathLibrary.MakeVector2D` _locationx _locationy) (`self.PreviousFingerPosition`)))))

(fn `FingerDistance`
  (returns (ReturnValue :type "Float (double-precision)"))
  (bind _returnvalue (`GameplayStatics.GetPlayerController` 0))
  (bind (_locationx _locationy) (`PlayerController.GetInputTouchState` _returnvalue "Touch2"))
  (bind (_locationx_2 _locationy_2) (`PlayerController.GetInputTouchState` _returnvalue "Touch1"))
  (return (`KismetMathLibrary.Distance2D` (`KismetMathLibrary.MakeVector2D` _locationx_2 _locationy_2) (`KismetMathLibrary.MakeVector2D` _locationx _locationy))))

(fn `GestureRecognition`
  (if (and (`self.ObjectIsPlaced`) (`self.FingerPressed`) (not (`self.GestureRecognize`)))
    (bind _output_get (set `self.FingerTimer` (+ (`self.Delta`) (`self.FingerTimer`))))
    (if (> _output_get 0.2)
      (set `self.GestureRecognize` true)
      (set `self.State` "NewEnumerator0"))
    (else
      (set `self.FingerTimer` 0.0))))

(fn `GestureReset`
  (if (`self.GestureRecognize`)
    (if (not (`.bIsCurrentlyPressed` (`PlayerController.GetInputTouchState` (`GameplayStatics.GetPlayerController` 0) "Touch1")))
      (bind _output_get (set `self.GestureResetTime` (+ (`self.Delta`) (`self.GestureResetTime`))))
      (if (> _output_get 0.1)
        (set `self.GestureRecognize` false)
        (set `self.GestureResetTime` 0.0))
      (else
        (set `self.GestureResetTime` 0.0)))))

(fn `ResetPlace`
  (bind _object (`self.Object`))
  (bind _selectedplane (`self.SelectedPlane`))
  (set `self.ObjectIsPlaced` false)
  (set `self.PlaneIsSelected` false)
  (`|ExecutionSequence`
    (:`then_0`
      (`/Engine/EditorBlueprintResources/StandardMacros.IsValid` _object
        (:`Is Valid`
          (`self.K2_DestroyActor` _object))))
    (:`then_1`
      (`/Engine/EditorBlueprintResources/StandardMacros.IsValid` _selectedplane
        (:`Is Valid`
          (`self.K2_DestroyActor` _selectedplane))))))

(fn `ScreenCenter`
  (returns (ReturnValue :type "Vector2D Structure"))
  (bind (_sizex _sizey) (`PlayerController.GetViewportSize` (`GameplayStatics.GetPlayerController` 0)))
  (return (* (`KismetMathLibrary.MakeVector2D` (`KismetMathLibrary.Conv_IntToDouble` _sizex) (`KismetMathLibrary.Conv_IntToDouble` _sizey)) 0.5)))

(fn `TouchLocation`
  (returns (Touch :type "Vector2D Structure"))
  (bind (_locationx _locationy) (`PlayerController.GetInputTouchState` (`GameplayStatics.GetPlayerController` 0) "Touch1"))
  (return (`KismetMathLibrary.MakeVector2D` _locationx _locationy)))

(fn `TwoTouch`
  (if (and (`self.TwoFingerPressed`) (`self.ObjectIsPlaced`) (not (`self.GestureRecognize`)))
    (bind _output_get (set `self.TwoFingerTimer` (+ (`self.Delta`) (`self.TwoFingerTimer`))))
    (if (> _output_get 0.2)
      (if (`KismetMathLibrary.NearlyEqual_FloatFloat` (`KismetMathLibrary.Abs` (- (`self.PreviousFingerDistance`) (`self.FingerDistance`))) 0.0 0.001)
        (set `self.TwoFingerTimer` 0.0)
        (else
          (set `self.GestureRecognize` true)
          (if (< (`KismetMathLibrary.Abs` (`.Y` (`KismetMathLibrary.BreakVector2D` (`self.FingerDirection`)))) 0.5)
            (set `self.State` "NewEnumerator1")))))
    (else
      (set `self.TwoFingerTimer` 0.0))))

(fn `Update`
  (bind _bp_planecandidate (`self.BP_PlaneCandidate`))
  (bind _returnvalue (`ARBlueprintLibrary.LineTraceTrackedObjects` (`self.ScreenCenter`) false false))
  (`/Engine/EditorBlueprintResources/StandardMacros.CompareInt` (`KismetArrayLibrary.Array_Length` _returnvalue)
    (:`>`
      (bind _asarplane_geometry (cast `ARPlaneGeometry` (`ARTraceResultLibrary.GetTrackedGeometry` (`|GetArrayItem` _returnvalue))))
      (bind _plane (`self.Create` _asarplane_geometry))
      (`/Engine/EditorBlueprintResources/StandardMacros.IsValid` _plane
        (:`Is Valid`
          (`|ExecutionSequence`
            (:`then_0`
              (`/Engine/EditorBlueprintResources/StandardMacros.IsValid` _bp_planecandidate
                (:`Is Valid`
                  (`self.K2_DestroyActor` _bp_planecandidate))))
            (:`then_1`
              (set `self.BP_PlaneCandidate` _plane))))))))

(fn `UserConstructionScript`)

(fn `WorldHit`
  (params (Location :type "Vector2D Structure"))
  (returns (OutHit :type "HitResult Structure") (ReturnValue :type Boolean))
  (bind (_worldposition _worlddirection) (`GameplayStatics.DeprojectScreenToWorld` (`GameplayStatics.GetPlayerController` 0) Location))
  (bind (_outhit _returnvalue) (`KismetSystemLibrary.LineTraceSingleForObjects` _worldposition (+ _worldposition (* _worlddirection 1000.0)) (`|MakeArray` "ObjectTypeQuery1" "ObjectTypeQuery2" "ObjectTypeQuery3" "ObjectTypeQuery4" "ObjectTypeQuery5" "ObjectTypeQuery6" :!type "EObjectTypeQuery Enum")))
  (return _outhit _returnvalue))